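; BP_SuperSpeed is a power-up that temporarily doubles the walk speed of the player who activates it.
; On activation it stores that player and sets the CharacterMovementComponent's MaxWalkSpeed to twice GetMaxSpeed.
; On expiry it sets MaxWalkSpeed to half the current GetMaxSpeed if the component is valid, then calls the parent's expiry logic.
; It caches no original speed, so restoration depends on GetMaxSpeed at expiry.
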(event EventOnExpired
  (bind _activedforplayer (Variables|Default|GetActivedForPlayer))
  (bind _returnvalue (Actor|GetComponentbyClass _activedforplayer "/Script/Engine.CharacterMovementComponent"))
  (Utilities|IsValid _returnvalue
    (:Is%20Valid
      (Variables|/Script/Engine.CharacterMovementComponent|SetMaxWalkSpeed _returnvalue (/ (Class|MovementComponent|GetMaxSpeed _returnvalue) 2.0)))
    (:Is%20Not%20Valid
      _))
  (|CallParentFunction))

(event EventOnActivated
  (params (ActivateFor :type Actor%20Object%20Reference))
  (bind _returnvalue (Actor|GetComponentbyClass ActivateFor "/Script/Engine.CharacterMovementComponent"))
  (Variables|Default|SetActivedForPlayer ActivateFor)
  (Variables|/Script/Engine.CharacterMovementComponent|SetMaxWalkSpeed _returnvalue (* (Class|MovementComponent|GetMaxSpeed _returnvalue) 2.0)))

(fn ConstructionScript)